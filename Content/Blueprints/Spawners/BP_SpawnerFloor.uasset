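; Floor spawner that lays a row of tiles along X and recycles them to form a continuous floor.
; On BeginPlay it spawns tiles through the parent's SpawnActor, placing the first at its own location and measuring tile size from that tile's bounds.
; Each following tile goes one tile size past RearTile.
; SpawnActorHitBounds moves out-of-bounds tiles behind RearTile and makes them the new rear, avoiding respawns.
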(event `self.ReceiveBeginPlay`
  (bind (_returnvalue_x _returnvalue_y) (`KismetMathLibrary.BreakVector` (`self.K2_GetActorLocation` (`self.RearTile`))))
  (for _index (range (+ (`self.NumActorsRequired`) 1))
    (if (== _index 0)
      (bind _returnvalue (`self.SpawnActor`))
      (bind _output_get (set `self.RearTile` _returnvalue))
      (set `self.TileSize` (* 2 (.x (`.BoxExtent` (`self.GetActorBounds` _returnvalue false false)))))
      (`self.K2_SetActorLocation` _output_get (`self.K2_GetActorLocation`) false false)
      (else
        (bind _returnvalue_2 (`self.SpawnActor`))
        (`self.K2_SetActorLocation` _returnvalue_2 (`KismetMathLibrary.MakeVector` (+ _returnvalue_x (`self.TileSize`)) _returnvalue_y) false false)
        (set `self.RearTile` _returnvalue_2)))))

(fn `SpawnActor`
  (returns (ReturnValue :type "Actor Object Reference"))
  (bind _returnvalue (`parent.SpawnActor`))
  (return _returnvalue))

(fn `SpawnActorHitBounds`
  (params (OutOfBoundsActor :type "Actor Object Reference"))
  (bind (_returnvalue_x _returnvalue_y) (`KismetMathLibrary.BreakVector` (`self.K2_GetActorLocation` (`self.RearTile`))))
  (`self.K2_SetActorLocation` OutOfBoundsActor (`KismetMathLibrary.MakeVector` (+ _returnvalue_x (`self.TileSize`)) _returnvalue_y) false false)
  (set `self.RearTile` OutOfBoundsActor))

(fn `UserConstructionScript`
  (`parent.UserConstructionScript`))