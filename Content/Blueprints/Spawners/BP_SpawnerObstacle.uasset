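; BP_SpawnerObstacle is a child spawner that produces obstacles at random intervals during play.
; On BeginPlay it finds the level manager and starts a self-rescheduling delay loop, which repeats while the manager reports the game is playing.
; Each cycle spawns an obstacle through the parent's SpawnActor and applies the spawner's location.
; Its SpawnActorHitBounds override destroys any out-of-bounds actor passed to it.
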(event `self.ReceiveBeginPlay`
  (bind (_levelmanager _bwaslevelmanagerfound) (`/Game/Blueprints/Libraries/BPF_Lib.GetLevelManager`))
  (if _bwaslevelmanagerfound
    (set `self.LevelManagerRef` _levelmanager)
    (`self.LineUpNextObstacleSpawn`)))

(event `LineUpNextObstacleSpawn`
  (`KismetSystemLibrary.Delay` (`KismetMathLibrary.RandomFloatInRange` (`self.MinDelay`) (`self.MaxDelay`)))
  (`self.PlaceObstacle`)
  (if (`/Game/Blueprints/Game/BP_LevelManager.bIsPlaying` (`self.LevelManagerRef`))
    (`self.LineUpNextObstacleSpawn`)))

(fn `PlaceObstacle`
  (`self.SpawnActor`)
  (`self.K2_SetActorLocation` (`self.K2_GetActorLocation`)))

(fn `SpawnActor`
  (returns (ReturnValue :type "Actor Object Reference"))
  (bind _returnvalue (`parent.SpawnActor`))
  (return _returnvalue))

(fn `SpawnActorHitBounds`
  (params (OutOfBoundsActor :type "Actor Object Reference"))
  (`self.K2_DestroyActor` OutOfBoundsActor))

(fn `UserConstructionScript`
  (`parent.UserConstructionScript`))