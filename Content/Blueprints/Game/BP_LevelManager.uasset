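; Level manager actor that controls game start and game over and holds the level speed and playing state.
; It shows the start menu on play and the game over widget on loss, passing itself to both and switching input mode and cursor to match.
; A LevelBounds box, sized and placed in the construction script, asks overlapping actors for their parent and notifies it via SpawnActorHitBounds.
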(event `self.ReceiveBeginPlay`
  (bind _returnvalue (`GameplayStatics.GetPlayerController` 0))
  (bind _returnvalue_2 (`|CreateWidget` "/Game/Blueprints/UI/WBP_StartMenu.WBP_StartMenu_C" null self))
  (`UserWidget.AddToViewport` _returnvalue_2 0)
  (`WidgetBlueprintLibrary.SetInputMode_UIOnlyEx` _returnvalue null)
  (set `PlayerController.bShowMouseCursor` true _returnvalue))

(event `self.LevelBounds.OnComponentBeginOverlap`
  (params (OverlappedComponent :type "PrimitiveComponent Object Reference") (OtherActor :type "Actor Object Reference") (OtherComp :type "PrimitiveComponent Object Reference") (OtherBodyIndex :type Integer) (bFromSweep :type Boolean) (SweepResult :type "HitResult Structure (by ref)"))
  (bind _parent (message `/Game/Blueprints/Misc/BPI_Spawnable.ReturnParent` OtherActor))
  (`/Engine/EditorBlueprintResources/StandardMacros.IsValid` _parent
    (:`Is Valid`
      (`/Game/Blueprints/Spawners/BP_SpawnerBase.SpawnActorHitBounds` _parent OtherActor))
    (:`Is Not Valid`
      (`KismetSystemLibrary.PrintString` "Hello"))))

(fn `GameOver`
  (bind _returnvalue (`GameplayStatics.GetPlayerController` 0))
  (set `self.LevelSpeed` 0.0)
  (set `self.bIsPlaying` false)
  (bind _returnvalue_2 (`|CreateWidget` "/Game/Blueprints/UI/WBP_GameOver.WBP_GameOver_C" null self))
  (`UserWidget.AddToViewport` _returnvalue_2 0)
  (`WidgetBlueprintLibrary.SetInputMode_UIOnlyEx` _returnvalue null)
  (set `PlayerController.bShowMouseCursor` true _returnvalue))

(fn `StartGame`
  (bind _returnvalue (`GameplayStatics.GetPlayerController` 0))
  (set `self.bIsPlaying` true)
  (`WidgetBlueprintLibrary.SetInputMode_GameOnly` _returnvalue)
  (set `PlayerController.bShowMouseCursor` false _returnvalue))

(fn `UserConstructionScript`
  (bind _levelbounds (`self.LevelBounds`))
  (`BoxComponent.SetBoxExtent` _levelbounds (`self.OutOfBoundBoxScale`) true)
  (`SceneComponent.K2_SetWorldLocation` _levelbounds (`self.OutOfBoundBoxLocation`) false false))