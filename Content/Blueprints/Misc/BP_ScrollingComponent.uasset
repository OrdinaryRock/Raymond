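; BP_ScrollingComponent is an actor component that scrolls its owning actor at the level's speed while the game is playing.
; On BeginPlay it caches the level manager if one is found.
; Each Tick, while that manager reports IsPlaying, it scales the owner's world forward vector by LevelSpeed and delta time.
; The result is applied as a local-space offset without sweep, so the owner's rotation affects it twice.
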(event `self.ReceiveBeginPlay`
  (bind (_levelmanager _bwaslevelmanagerfound) (`/Game/Blueprints/Libraries/BPF_Lib.GetLevelManager`))
  (if _bwaslevelmanagerfound
    (set `self.LevelManagerRef` _levelmanager)))

(event `self.ReceiveTick`
  (params (DeltaSeconds :type "Float (single-precision)"))
  (bind _returnvalue (`self.GetOwner`))
  (bind _levelmanagerref (`self.LevelManagerRef`))
  (bind _output_get (set `self.Delta Seconds` DeltaSeconds))
  (`/Engine/EditorBlueprintResources/StandardMacros.IsValid` _levelmanagerref
    (:`Is Valid`
      (if (`/Game/Blueprints/Game/BP_LevelManager.bIsPlaying` _levelmanagerref)
        (bind _output_get_2 (set `self.Movement` (* (* (`Actor.GetActorForwardVector` _returnvalue) (`/Game/Blueprints/Game/BP_LevelManager.LevelSpeed` (`self.LevelManagerRef`))) _output_get)))
        (`Actor.K2_AddActorLocalOffset` _returnvalue _output_get_2 false false)))))